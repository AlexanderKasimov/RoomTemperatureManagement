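; Door actor that swings open and closed in instant 90-degree steps when its Use event fires.
; A FlipFlop alternates the root's world yaw in each direction and stores its state in Open.
; On BeginPlay, a debug-drawn, zero-length sphere trace beside the mesh, offset along its negative right vector, looks for WorldDynamic objects and prints any hit actor's name.
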(event `self.ReceiveBeginPlay`
  (bind _staticmesh (`self.StaticMesh`))
  (bind _returnvalue (+ (`SceneComponent.K2_GetComponentLocation` _staticmesh) (* (`SceneComponent.GetRightVector` _staticmesh) -400.0)))
  (bind (_outhit _returnvalue_2) (`KismetSystemLibrary.SphereTraceSingleForObjects` :`Start` _returnvalue :`End` _returnvalue :`Radius` 30.0 :`ObjectTypes` (`|MakeArray` "ObjectTypeQuery2" :!type "EObjectTypeQuery Enum") :`bTraceComplex` true :`DrawDebugType` "ForDuration"))
  (if _returnvalue_2
    (`KismetSystemLibrary.PrintString` (`KismetSystemLibrary.GetDisplayName` (`.HitActor` (`GameplayStatics.BreakHitResult` _outhit))))))

(event `/Game/Blueprints/i_Interactable.Use`
  (bind _defaultsceneroot (`self.DefaultSceneRoot`))
  (bind _defaultsceneroot_2 (`self.DefaultSceneRoot`))
  (bind _isa (`/Engine/EditorBlueprintResources/StandardMacros.FlipFlop`)
    (:`A`
      (`SceneComponent.K2_SetWorldRotation` _defaultsceneroot (`KismetMathLibrary.MakeRotator` (.roll (`SceneComponent.K2_GetComponentRotation` _defaultsceneroot)) (.pitch (`SceneComponent.K2_GetComponentRotation` _defaultsceneroot)) (- (.yaw (`SceneComponent.K2_GetComponentRotation` _defaultsceneroot)) -90.0)) false false))
    (:`B`
      (`SceneComponent.K2_SetWorldRotation` _defaultsceneroot_2 (`KismetMathLibrary.MakeRotator` (.roll (`SceneComponent.K2_GetComponentRotation` _defaultsceneroot_2)) (.pitch (`SceneComponent.K2_GetComponentRotation` _defaultsceneroot_2)) (- (.yaw (`SceneComponent.K2_GetComponentRotation` _defaultsceneroot_2)) 90.0)) false false)))
  (set `self.Open` _isa))

(fn `UserConstructionScript`)