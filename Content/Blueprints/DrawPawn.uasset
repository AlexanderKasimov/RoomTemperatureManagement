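; DrawPawn is a Pawn that moves from player input through a FloatingPawnMovement component.
; The MoveForward and MoveRight axis events scale the control rotation's forward and right vectors by the axis value and feed them to the component as input vectors.
; Forward movement uses the full control rotation, so it follows pitch as well as yaw.
; The graphs contain no drawing or look-input logic.
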(event `InputAxis|MoveForward`
  (params (AxisValue :type "Float (single-precision)"))
  (`PawnMovementComponent.AddInputVector` (`self.FloatingPawnMovement`) (* (`KismetMathLibrary.GetForwardVector` (`self.GetControlRotation`)) AxisValue) false))

(event `InputAxis|MoveRight`
  (params (AxisValue :type "Float (single-precision)"))
  (`PawnMovementComponent.AddInputVector` (`self.FloatingPawnMovement`) (* (`KismetMathLibrary.GetRightVector` (`self.GetControlRotation`)) AxisValue) false))

(fn `UserConstructionScript`)