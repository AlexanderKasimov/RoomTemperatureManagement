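; DrawController is a player controller that sets up mouse-driven interaction and an on-screen temperature UI.
; On BeginPlay it shows the mouse cursor and adds a UI_Temperature widget to the viewport.
; A left click runs a complex Visibility trace under the cursor and calls UseMessage on the hit actor if it implements I_Interactable.
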(event `self.ReceiveBeginPlay`
  (set `self.bShowMouseCursor` true)
  (bind _returnvalue (`|CreateWidget` "/Game/UI/UI_Temperature.UI_Temperature_C" self))
  (`UserWidget.AddToViewport` _returnvalue 0))

(event `Key|LeftMouseButton`
  (params (Key :type "Key Structure"))
  (bind (_bblockinghit _binitialoverlap _time _location _impactpoint _normal _impactnormal _physmat _hitactor) (`GameplayStatics.BreakHitResult` (`self.GetHitResultUnderCursorByChannel` "TraceTypeQuery1")))
  (:`Pressed`
    (if (`KismetSystemLibrary.DoesImplementInterface` _hitactor "/Game/Blueprints/i_Interactable.i_Interactable_C")
      (message `/Game/Blueprints/i_Interactable.Use` _hitactor))))

(fn `UserConstructionScript`)