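; Room actor that simulates a temperature shared through open doors and shows it on a thermometer widget.
; Its construction script sizes the Box from the room dimensions and adds the widget and a child actor relative to it.
; BeginPlay caches every BP_Door that references this room on either side.
; Each Tick, open doors instantly set its temperature to the neighboring Room's, or the GameMode's OutsideTemp when the door's left side is empty.
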(event `self.ReceiveBeginPlay`
  (`|ExecutionSequence`
    (:`then_0`
      (bind _asui_thermometer (cast `/Game/UI/UI_Thermometer` (`WidgetComponent.GetUserWidgetObject` (`self.TermometerWidget`))))
      (set `self.UI_Thermometer` _asui_thermometer))
    (:`then_1`
      (bind _outactors (`GameplayStatics.GetAllActorsOfClass` "/Game/Blueprints/BP_Door.BP_Door_C"))
      (for _array_element _outactors
        (if (or (== (`/Game/Blueprints/BP_Door.LeftSideEnv` _array_element) self) (== (`/Game/Blueprints/BP_Door.RightSideEnv` _array_element) self))
          (`KismetArrayLibrary.Array_Add` (`self.DoorsConnected`) _array_element))))))

(event `self.ReceiveTick`
  (params (DeltaSeconds :type "Float (single-precision)"))
  (bind _returnvalue (+ (`self.RoomTemperature`) (+ (`self.OutsideTemp`) (* (`self.RoomTemperature`) -1.0))))
  (for _array_element (`self.DoorsConnected`)
    (if (`/Game/Blueprints/BP_Door.Open` _array_element)
      (`|ExecutionSequence`
        (:`then_0`
          (bind _leftsideenv (`/Game/Blueprints/BP_Door.LeftSideEnv` _array_element))
          (`/Engine/EditorBlueprintResources/StandardMacros.IsValid` _leftsideenv
            (:`Is Valid`
              (if (== _leftsideenv self)
                (bind _asroom (cast `/Game/Blueprints/Room` (`/Game/Blueprints/BP_Door.RightSideEnv` _array_element)))
                (bind _returnvalue_2 (+ (`self.RoomTemperature`) (+ (`/Game/Blueprints/Room.RoomTemperature` _asroom) (* (`self.RoomTemperature`) -1.0))))
                (set `/Game/UI/UI_Thermometer.RoomTemp` _returnvalue_2 (`self.UI_Thermometer`))
                (set `self.RoomTemperature` _returnvalue_2)
                (else
                  (bind _asroom_2 (cast `/Game/Blueprints/Room` _leftsideenv))
                  (bind _returnvalue_3 (+ (`self.RoomTemperature`) (+ (`/Game/Blueprints/Room.RoomTemperature` _asroom_2) (* (`self.RoomTemperature`) -1.0))))
                  (set `/Game/UI/UI_Thermometer.RoomTemp` _returnvalue_3 (`self.UI_Thermometer`))
                  (set `self.RoomTemperature` _returnvalue_3))))
            (:`Is Not Valid`
              (bind _asroom_temperature_game_mode (cast `/Game/Blueprints/RoomTemperatureGameMode` (`GameplayStatics.GetGameMode`)))
              (set `self.OutsideTemp` (`/Game/Blueprints/RoomTemperatureGameMode.OutsideTemp` _asroom_temperature_game_mode))
              (set `/Game/UI/UI_Thermometer.RoomTemp` _returnvalue (`self.UI_Thermometer`))
              (set `self.RoomTemperature` _returnvalue))))))))

(fn `UserConstructionScript`
  (`|ExecutionSequence`
    (:`then_0`
      (`BoxComponent.SetBoxExtent` (`self.Box`) (`KismetMathLibrary.MakeVector` (/ (`self.SizeX`) 2.0) (/ (`self.SizeY`) 2.0) (/ (`self.SizeZ`) 2.0)) true))
    (:`then_1`
      (bind _returnvalue (`AddComponent|NODE_AddWidgetComponent-0` :`RelativeTransform` (`KismetMathLibrary.MakeTransform` (`KismetMathLibrary.MakeVector` 0.0 0.0 (- (.z (.location (`SceneComponent.GetRelativeTransform` (`self.Box`)))) (/ (`self.SizeZ`) 2.0))) (struct :`Pitch` 90.0 :`Roll` 180.0))))
      (set `self.TermometerWidget` _returnvalue))
    (:`then_2`
      (`AddComponent|NODE_AddChildActorComponent-0` :`RelativeTransform` (`KismetMathLibrary.MakeTransform` (`KismetMathLibrary.MakeVector` 0.0 (+ (.y (.location (`SceneComponent.GetRelativeTransform` (`self.Box`)))) (/ (`self.SizeY`) -2.0) 0.0) (- (.z (.location (`SceneComponent.GetRelativeTransform` (`self.Box`)))) (/ (`self.SizeZ`) 2.0))) (struct))))))